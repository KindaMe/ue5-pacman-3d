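; BP_Pawn_Pacman is the common Pac-Man pawn, able to harm frightened ghosts and report its death state to the game mode.
; When its capsule overlaps a ghost in Frightened mode, it applies its current damage to that ghost.
; Its SetIsDead override runs the parent logic, then notifies the game mode through the BPI_Pawns interface.
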(event OnComponentBeginOverlap(CapsuleCollision)
  (params (OverlappedComponent :type Primitive%20Component%20Object%20Reference) (OtherActor :type Actor%20Object%20Reference) (OtherComp :type Primitive%20Component%20Object%20Reference) (OtherBodyIndex :type Integer) (bFromSweep :type Boolean) (SweepResult :type Hit%20Result%20Structure%20%28by%20ref%29))
  (bind _asbp_pawn_ghost (Utilities|Casting|CastToBP_Pawn_Ghost OtherActor))
  (switch Utilities|FlowControl|Switch|SwitchonE_GhostModes (Default|GetCurrentMode _asbp_pawn_ghost)
    (:NewEnumerator2
      (Game|Damage|ApplyDamage _asbp_pawn_ghost (Math|Conversions|ToFloat(Integer) (CallFunction|GetCurrentDamage)) 0 0))))

(fn ConstructionScript
  (|CallParentFunction))

(fn SetIsDead
  (params (IsDead :type Boolean))
  (bind _returnvalue (Game|GetGameMode))
  (|CallParentFunction IsDead)
  (if (Utilities|DoesObjectImplementInterface _returnvalue "/Game/PacmanGame/Characters/BPI_Pawns.BPI_Pawns_C")
    (Class|BPIPawns|OnPacmanIsDead(Message) _returnvalue self IsDead)))