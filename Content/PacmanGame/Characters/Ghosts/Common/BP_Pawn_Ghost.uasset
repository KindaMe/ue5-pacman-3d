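; BP_Pawn_Ghost is a ghost pawn for a Pacman game that configures its AI behavior on BeginPlay.
; It gets the AI controller's Behavior Tree component and injects the ScatterBT, FrightenedBT and ChaseBT assets as dynamic subtrees under matching gameplay tags.
; This lets a behavior tree with tagged subtree slots run different scatter, frightened and chase logic according to the assets set on the ghost.
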(event EventBeginPlay
  (bind _self self)
  (bind _returnvalue (AI|GetAIController _self))
  (Utilities|IsValid _returnvalue
    (:Is%20Valid
      (bind _asbehavior_tree_component (Utilities|Casting|CastToBehaviorTreeComponent (Variables|/Script/AIModule.AIController|GetBrainComponent _returnvalue)))
      (Class|BehaviorTreeComponent|SetDynamicSubtree _asbehavior_tree_component "(TagName=\"GhostScatter\")" (Variables|Default|GetScatterBT))
      (Class|BehaviorTreeComponent|SetDynamicSubtree _asbehavior_tree_component "(TagName=\"GhostFrightened\")" (Variables|Default|GetFrightenedBT))
      (Class|BehaviorTreeComponent|SetDynamicSubtree _asbehavior_tree_component "(TagName=\"GhostChase\")" (Variables|Default|GetChaseBT)))))

(fn ConstructionScript
  (|CallParentFunction))