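; Base pawn for the Pac-Man game that holds health, speed, damage, death state and mesh material.
; Construction resets each stat and the material to defaults through setter functions, which clamp health and damage at zero and push speed into FloatingPawnMovement's MaxSpeed.
; AnyDamage subtracts from health and flags the pawn dead at zero.
; Clearing the dead flag restores default health.
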(event Game|Damage|EventAnyDamage
  (params (Damage :type Float%20%28single-precision%29) (DamageType :type Damage%20Type%20Object%20Reference) (InstigatedBy :type Controller%20Object%20Reference) (DamageCauser :type Actor%20Object%20Reference))
  (bind _currenthealth (CallFunction|GetCurrentHealth))
  (CallFunction|SetCurrentHealth (Math|Integer|Max(Integer) (- _currenthealth Damage)))
  (if (== 0 _currenthealth)
    (CallFunction|SetIsDead true)))

(fn ConstructionScript
  (CallFunction|ResetCurrentSpeed)
  (CallFunction|ResetCurrentHealth)
  (CallFunction|ResetCurrentDamage)
  (CallFunction|ResetMeshMaterial))

(fn GetCurrentHealth
  (return (Variables|Default|GetCurrentHealth)))

(fn SetCurrentHealth
  (params (NewHealth :type Integer))
  (Variables|Default|SetCurrentHealth (Math|Integer|Max(Integer) NewHealth))
  (return))

(fn ResetCurrentHealth
  (CallFunction|SetCurrentHealth (Variables|Default|GetDefaultHealth))
  (return))

(fn AddCurrentHealth
  (params (AddHealth :type Integer))
  (CallFunction|SetCurrentHealth (+ AddHealth (CallFunction|GetCurrentHealth)))
  (return))

(fn GetCurrentSpeed
  (return (Variables|Default|GetCurrentSpeed)))

(fn SetCurrentSpeed
  (params (NewSpeed :type Float%20%28double-precision%29))
  (bind _output_get (Variables|Default|SetCurrentSpeed NewSpeed))
  (Variables|/Script/Engine.FloatingPawnMovement|SetMaxSpeed (Variables|Default|GetFloatingPawnMovement) _output_get)
  (return))

(fn ResetCurrentSpeed
  (CallFunction|SetCurrentSpeed (Variables|Default|GetDefaultSpeed))
  (return))

(fn GetCurrentDamage
  (return (Variables|Default|GetCurrentDamage)))

(fn SetCurrentDamage
  (params (CurrentDamage :type Integer))
  (Variables|Default|SetCurrentDamage (Math|Integer|Max(Integer) CurrentDamage))
  (return))

(fn ResetCurrentDamage
  (CallFunction|SetCurrentDamage (Variables|Default|GetDefaultDamage))
  (return))

(fn SetIsDead
  (params (IsDead :type Boolean))
  (bind _output_get (Variables|Default|SetIsDead IsDead))
  (if _output_get
    _
    (else
      (CallFunction|ResetCurrentHealth)))
  (return))

(fn SetMeshMaterial
  (params (NewMaterial :type Material%20Interface%20Object%20Reference))
  (Rendering|Material|SetMaterial (Variables|Default|GetStaticMesh) 0 NewMaterial))

(fn ResetMeshMaterial
  (CallFunction|SetMeshMaterial (Variables|Default|GetDefaultStaticMeshMaterial)))