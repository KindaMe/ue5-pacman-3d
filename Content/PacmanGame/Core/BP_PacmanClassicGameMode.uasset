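; BP_PacmanClassicGameMode is the game mode that sets up a classic Pac-Man session.
; On BeginPlay it spawns a BP_Maze_Game from the last maze template stored in BP_GameInstance.
; It then possesses the maze's first player pawn with the controller captured in PostLogin and switches that controller's view target to the maze actor.
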(event Custom|PossessPawns
  (Pawn|Possess (Variables|Default|GetPlayerControllerRef) (Utilities|Array|Get(acopy) (Variables|/Game/PacmanGame/Maze/BP_Maze.BP_Maze_C|GetPlayerPawns (Variables|Default|GetMazeRef)))))

(event EventBeginPlay
  (bind _asbp_game_instance (Utilities|Casting|CastToBP_GameInstance (Game|GetGameInstance)))
  (bind _returnvalue (Game|SpawnActorfromClass "/Game/PacmanGame/Maze/BP_Maze_Game.BP_Maze_Game_C" (Math|Transform|MakeTransform "0, 0, 0" "0, 0, 0" "1.000000,1.000000,1.000000") "AlwaysSpawn" "MultiplyWithRoot" 0 (Utilities|Array|Get(acopy) (Variables|/Game/PacmanGame/Core/BP_GameInstance.BP_GameInstance_C|GetMazes _asbp_game_instance) (Utilities|Array|LastIndex (Variables|/Game/PacmanGame/Core/BP_GameInstance.BP_GameInstance_C|GetMazes _asbp_game_instance))) 100 0))
  (Variables|Default|SetMazeRef _returnvalue)
  (CallFunction|PossessPawns)
  (Game|Player|SetViewTargetwithBlend (Variables|Default|GetPlayerControllerRef) (Variables|Default|GetMazeRef) 0.0 "VTBlend_Linear" 0.0 false))

(event EventPostLogin
  (params (NewPlayer :type Player%20Controller%20Object%20Reference))
  (Variables|Default|SetPlayerControllerRef NewPlayer))

(fn ConstructionScript)