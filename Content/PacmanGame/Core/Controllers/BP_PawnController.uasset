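; Player controller for the Pac-Man game that turns player input into movement on the possessed BP_Pawn.
; On BeginPlay it adds the in-game Enhanced Input mapping context, and on possession it caches the pawn.
; The move action feeds its X/Y value to that pawn as world-direction movement input.
; Debug keys Z, X, C and V force every ghost into Scatter, Chase, Frightened or Dead mode, printing the mode name.
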(event Input|EnhancedActionEvents|EnhancedInputActionIA_Move
  (params (ActionValue :type Vector%202D%20Structure) (ElapsedSeconds :type Float%20%28double-precision%29) (TriggeredSeconds :type Float%20%28double-precision%29) (InputAction :type Input%20Action%20Object%20Reference :default "/Game/PacmanGame/Core/IMCs/Actions/IA_Move.IA_Move"))
  (bind _possessedpawn (Variables|Default|GetPossessedPawn))
  (:Triggered
    (Utilities|IsValid _possessedpawn
      (:Is%20Valid
        (Pawn|Input|AddMovementInput _possessedpawn (Math|Vector|MakeVector (.x ActionValue) (.y ActionValue) 0.0) 1.0 false)))))

(event EventPossess
  (params (PossessedPawn :type Pawn%20Object%20Reference))
  (bind _asbp_pawn (Utilities|Casting|CastToBP_Pawn PossessedPawn))
  (Variables|Default|SetPossessedPawn _asbp_pawn))

(event EventBeginPlay
  (bind _returnvalue (PlayerController|LocalPlayerSubsystems|GetEnhancedInputLocalPlayerSubsystem))
  (Utilities|IsValid _returnvalue
    (:Is%20Valid
      (Input|AddMappingContext _returnvalue "/Game/PacmanGame/Core/IMCs/IMC_InGame.IMC_InGame" 0 "(bIgnoreAllPressedKeysUntilRelease=True,bForceImmediately=False)"))))

(event Input|KeyboardEvents|Z
  (params (Key :type Key%20Structure :default "None"))
  ;[1 1 1] debug
  (:Pressed
    (bind _outactors (Actor|GetAllActorsOfClass "/Game/PacmanGame/Characters/Ghosts/Common/BP_Pawn_Ghost.BP_Pawn_Ghost_C"))
    (for _array_element _outactors
      (Default|ChangeMode _array_element "NewEnumerator0"))
    (Development|PrintString "Scatter")))

(event Input|KeyboardEvents|X
  (params (Key :type Key%20Structure :default "None"))
  ;[1 1 1] debug
  (:Pressed
    (bind _outactors (Actor|GetAllActorsOfClass "/Game/PacmanGame/Characters/Ghosts/Common/BP_Pawn_Ghost.BP_Pawn_Ghost_C"))
    (for _array_element _outactors
      (Default|ChangeMode _array_element "NewEnumerator1"))
    (Development|PrintString "Chase")))

(event Input|KeyboardEvents|C
  (params (Key :type Key%20Structure :default "None"))
  ;[1 1 1] debug
  (:Pressed
    (bind _outactors (Actor|GetAllActorsOfClass "/Game/PacmanGame/Characters/Ghosts/Common/BP_Pawn_Ghost.BP_Pawn_Ghost_C"))
    (for _array_element _outactors
      (Default|ChangeMode _array_element "NewEnumerator2"))
    (Development|PrintString "Frightened")))

(event Input|KeyboardEvents|V
  (params (Key :type Key%20Structure :default "None"))
  ;[1 1 1] debug
  (:Pressed
    (bind _outactors (Actor|GetAllActorsOfClass "/Game/PacmanGame/Characters/Ghosts/Common/BP_Pawn_Ghost.BP_Pawn_Ghost_C"))
    (for _array_element _outactors
      (Default|ChangeMode _array_element "NewEnumerator3"))
    (Development|PrintString "Dead")))

(fn ConstructionScript)