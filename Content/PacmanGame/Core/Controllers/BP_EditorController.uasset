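; Player controller for the maze editor, where the player builds a custom maze and saves it to the game instance.
; The editor widget's size event spawns a replacement maze actor as the view target, while saving stores its cells and loads the menu.
; Enhanced Input pans and zooms the maze's spring arm within maze-sized bounds.
; Clicks trace under the cursor and set the selected cell class through BPI_Cell on the hit actor or its parent.
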(event Custom|OnSave_Event
  (params (Name :type Text))
  (bind _asbp_game_instance (Utilities|Casting|CastToBP_GameInstance (Game|GetGameInstance)))
  (bind _refreshedmaze (Default|RefreshMazeTemplate (Variables|Default|GetMazeRef)))
  (Default|AddMaze _asbp_game_instance (Utilities|Struct|MakeS_Maze Name (.Width (Utilities|Struct|BreakS_Maze _refreshedmaze)) (.Height (Utilities|Struct|BreakS_Maze _refreshedmaze)) (.Cells (Utilities|Struct|BreakS_Maze _refreshedmaze))))
  (Default|LoadMenuLevel _asbp_game_instance))

(event Custom|OnSizeSet_Event
  (params (Width :type Integer) (Height :type Integer))
  (bind _returnvalue (Game|SpawnActorfromClass "/Game/PacmanGame/Maze/BP_Maze_Editor.BP_Maze_Editor_C" (Math|Transform|MakeTransform "0, 0, 0" "0, 0, 0" "1.000000,1.000000,1.000000") "AlwaysSpawn" "MultiplyWithRoot" 0 Width Height 100 0))
  (Utilities|IsValid (Variables|Default|GetMazeRef)
    (:Is%20Valid
      (Actor|DestroyActor (Variables|Default|GetMazeRef)))
    (:Is%20Not%20Valid
      _))
  (bind _output_get (Variables|Default|SetMazeRef _returnvalue))
  (Game|Player|SetViewTargetwithBlend _output_get 0.0 "VTBlend_Linear" 0.0 false)
  (CallFunction|AddMappingContext))

(event Custom|AddMappingContext
  (bind _returnvalue (PlayerController|LocalPlayerSubsystems|GetEnhancedInputLocalPlayerSubsystem))
  (Utilities|IsValid _returnvalue
    (:Is%20Valid
      (if (not (.ReturnValue (Class|EnhancedInputSubsystemInterface|HasMappingContext _returnvalue "/Game/PacmanGame/Core/IMCs/IMC_MazeEditor.IMC_MazeEditor")))
        (Input|AddMappingContext _returnvalue "/Game/PacmanGame/Core/IMCs/IMC_MazeEditor.IMC_MazeEditor" 0 "(bIgnoreAllPressedKeysUntilRelease=True,bForceImmediately=False)")))))

(event Custom|ChangeSelectedMazeComponent
  (params (NewCell :type BP%20Maze%20Cell%20Class%20Reference))
  (bind _output_get (Variables|Default|SetCurrentlySelectedCell NewCell))
  (Development|PrintString (Utilities|GetClassDisplayName _output_get)))

(event Input|EnhancedActionEvents|EnhancedInputActionIA_Zoom
  (params (ActionValue :type Float%20%28double-precision%29) (ElapsedSeconds :type Float%20%28double-precision%29) (TriggeredSeconds :type Float%20%28double-precision%29) (InputAction :type Input%20Action%20Object%20Reference :default "/Game/PacmanGame/Core/IMCs/Actions/IA_Zoom.IA_Zoom"))
  (bind _mazeref (Variables|Default|GetMazeRef))
  (bind _mazeref_2 (Variables|Default|GetMazeRef))
  (bind _maze (Variables|/Game/PacmanGame/Core/Maze/BP_Maze.BP_Maze_C|GetMaze _mazeref))
  (bind _springarm (Variables|/Game/PacmanGame/Core/Maze/BP_Maze.BP_Maze_C|GetSpringArm _mazeref_2))
  (bind (_name _width _height) (Utilities|Struct|BreakS_Maze _maze))
  (:Triggered
    (Utilities|IsValid _mazeref_2
      (:Is%20Valid
        (Variables|/Script/Engine.SpringArmComponent|SetTargetArmLength _springarm (Math|Float|Clamp(Float) (- (Variables|/Script/Engine.SpringArmComponent|GetTargetArmLength _springarm) (* ActionValue (Variables|Default|GetScrollSpeed))) 3e+02 (* (Math|Conversions|ToFloat(Integer) (Math|Integer|Max(Integer) (* _width 100) (* _height 100))) 1.5)))))))

(event Input|EnhancedActionEvents|EnhancedInputActionIA_ResetView
  (params (ActionValue :type Boolean) (ElapsedSeconds :type Float%20%28double-precision%29) (TriggeredSeconds :type Float%20%28double-precision%29) (InputAction :type Input%20Action%20Object%20Reference :default "/Game/PacmanGame/Core/IMCs/Actions/IA_ResetView.IA_ResetView"))
  (bind _mazeref (Variables|Default|GetMazeRef))
  (:Started
    (Utilities|IsValid _mazeref
      (:Is%20Valid
        (Default|ResetCameraLocation _mazeref)))))

(event Input|EnhancedActionEvents|EnhancedInputActionIA_Move
  (params (ActionValue :type Vector%202D%20Structure) (ElapsedSeconds :type Float%20%28double-precision%29) (TriggeredSeconds :type Float%20%28double-precision%29) (InputAction :type Input%20Action%20Object%20Reference :default "/Game/PacmanGame/Core/IMCs/Actions/IA_Move.IA_Move"))
  (bind _returnvalue (Math|Vector|MakeVector (.x ActionValue) (.y ActionValue) 0.0))
  (bind _returnvalue_2 (Utilities|Time|GetWorldDeltaSeconds))
  (bind _movespeed (Variables|Default|GetMoveSpeed))
  (bind _mazeref (Variables|Default|GetMazeRef))
  (bind _mazeref_2 (Variables|Default|GetMazeRef))
  (bind _returnvalue_3 (Math|Vector|Normalize _returnvalue))
  (bind _returnvalue_4 (* _movespeed _returnvalue_2))
  (bind _springarm (Variables|/Game/PacmanGame/Core/Maze/BP_Maze.BP_Maze_C|GetSpringArm _mazeref))
  (bind _maze (Variables|/Game/PacmanGame/Core/Maze/BP_Maze.BP_Maze_C|GetMaze _mazeref_2))
  (bind (_name _width _height) (Utilities|Struct|BreakS_Maze _maze))
  (bind _returnvalue_5 (* _returnvalue_3 _returnvalue_4))
  (bind _relativelocation (Variables|/Script/Engine.SceneComponent|GetRelativeLocation _springarm))
  (bind _returnvalue_6 (+ _returnvalue_5 _relativelocation))
  (:Triggered
    (Utilities|IsValid _mazeref
      (:Is%20Valid
        (Transformation|SetRelativeLocation _springarm (Math|Vector|MakeVector (Math|Float|Clamp(Float) (.x _returnvalue_6) 0.0 (Math|Conversions|ToFloat(Integer) (* (- _height 1) 100))) (Math|Float|Clamp(Float) (.y _returnvalue_6) 0.0 (Math|Conversions|ToFloat(Integer) (* (- _width 1) 100))) 0.0) false false)))))

(event Input|EnhancedActionEvents|EnhancedInputActionIA_Click
  (params (ActionValue :type Boolean) (ElapsedSeconds :type Float%20%28double-precision%29) (TriggeredSeconds :type Float%20%28double-precision%29) (InputAction :type Input%20Action%20Object%20Reference :default "/Game/PacmanGame/Core/IMCs/Actions/IA_Click.IA_Click"))
  (bind (_worldlocation _worlddirection) (Game|Player|ConvertMouseLocationToWorldSpace))
  (:Triggered
    (Utilities|IsValid (Variables|Default|GetMazeRef)
      (:Is%20Valid
        (bind (_outhit _returnvalue) (Collision|LineTraceByChannel _worldlocation (+ _worldlocation (* _worlddirection 100000)) "TraceTypeQuery2" true 0 "None"))
        (if _returnvalue
          (if (Utilities|DoesObjectImplementInterface (.hitactor _outhit) "/Game/PacmanGame/Maze/BPI_Cell.BPI_Cell_C")
            (bind _updated_ (Class|BPICell|SetChildActorClass(Message) (.hitactor _outhit) (Variables|Default|GetCurrentlySelectedCell)))
            (if _updated_
              (Development|PrintString "Updated Cell" :!label _label))
            (elif (Utilities|DoesObjectImplementInterface (Actor|GetParentActor (.hitactor _outhit)) "/Game/PacmanGame/Maze/BPI_Cell.BPI_Cell_C")
              (bind _updated__2 (Class|BPICell|SetChildActorClass(Message) (Actor|GetParentActor (.hitactor _outhit)) (Variables|Default|GetCurrentlySelectedCell)))
              (if _updated__2
                (goto _label)))))))))

(event EventBeginPlay
  (bind _returnvalue (UserInterface|CreateWidget "/Game/PacmanGame/UI/WBP_Editor.WBP_Editor_C" self))
  (bind _output_get (Variables|Default|SetEditorWidgetRef _returnvalue))
  (EventDispatchers|AssignOnSizeSet _output_get (delegate Custom|OnSizeSet_Event))
  (UserInterface|Viewport|AddtoViewport _output_get 0)
  (Input|SetInputModeGameandUI self _output_get "DoNotLock" false false)
  (Variables|Default|SetbShowMouseCursor true)
  (EventDispatchers|AssignOnSave _output_get (delegate Custom|OnSave_Event)))

(fn ConstructionScript)