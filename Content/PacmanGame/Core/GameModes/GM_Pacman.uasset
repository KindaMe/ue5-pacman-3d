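; Base-style Pacman game mode that handles pawn possession, score and default game states, and creates the in-game widget on player login.
; InitGame runs PreGame, which shows START and waits the returned duration, then InGame, which immediately calls PostGame as a win.
; Pickup collection adds non-negative score and refreshes the widget.
; Helpers possess or release Pacman and ghost pawns and store the default maze template.
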(event Custom|PossessPacman
  (params (PacmanPawn :type BP%20Pawn%20Pacman%20Object%20Reference))
  ;[1 1 1] possess/unpossess pacman/ghosts
  (Pawn|Possess (Variables|Default|GetPlayerControllerRef) PacmanPawn))

(event Custom|PreGame
  ;[1 1 1] default game states
  (bind _totalpredictedtime (CallFunction|DisplayAnimatedTextonScreen (Utilities|Array|MakeArray (Utilities|Struct|MakeS_AnimatedTextEntry "START" 0.0 1.0 "(R=1.000000,G=1.000000,B=1.000000,A=1.000000)"))))
  (Utilities|FlowControl|Delay _totalpredictedtime)
  (CallFunction|InGame))

(event Custom|UnPossessGhosts
  (params (GhostPawns :type Array%20of%20BP%20Pawn%20Ghost%20Object%20References))
  ;[1 1 1] possess/unpossess pacman/ghosts
  (for _array_element GhostPawns
    (Utilities|IsValid (AI|GetAIController _array_element)
      (:Is%20Valid
        (Pawn|UnPossess (AI|GetAIController _array_element))))))

(event Custom|InitGame
  ;[1 1 1] default game states
  (CallFunction|PreGame))

(event Custom|PossessGhosts
  (params (GhostPawns :type Array%20of%20BP%20Pawn%20Ghost%20Object%20References))
  ;[1 1 1] possess/unpossess pacman/ghosts
  (Pawn|SpawnDefaultController GhostPawns))

(event Custom|PostGame
  (params (IsWin? :type Boolean))
  ;[1 1 1] default game states
  (if IsWin?
    (CallFunction|DisplayAnimatedTextonScreen (Utilities|Array|MakeArray (Utilities|Struct|MakeS_AnimatedTextEntry "WIN" 0.0 1.0 "(R=0.000000,G=1.000000,B=0.000000,A=1.000000)")))
    (else
      (CallFunction|DisplayAnimatedTextonScreen (Utilities|Array|MakeArray (Utilities|Struct|MakeS_AnimatedTextEntry "LOSE" 0.0 1.0 "(R=0.995000,G=0.000000,B=0.000000,A=1.000000)"))))))

(event Custom|InGame
  ;[1 1 1] default game states
  (CallFunction|PostGame true))

(event Custom|UnPossessPacman
  ;[1 1 1] possess/unpossess pacman/ghosts
  (Pawn|UnPossess (Variables|Default|GetPlayerControllerRef)))

(event EventBeginPlay
  ;[1 1 1] begin play
  (bind _asbp_game_instance (Utilities|Casting|CastToBP_GameInstance (Game|GetGameInstance)))
  (Variables|Default|SetGameInstanceRef _asbp_game_instance))

(event EventPostLogin
  (params (NewPlayer :type Player%20Controller%20Object%20Reference))
  ;[1 1 1] onpostlogin
  (bind _asbp_pawn_controller (Utilities|Casting|CastToBP_PawnController NewPlayer))
  (Variables|Default|SetPlayerControllerRef _asbp_pawn_controller)
  (bind _returnvalue (UserInterface|CreateWidget "/Game/PacmanGame/UI/InGame/WBP_InGame.WBP_InGame_C"))
  (bind _output_get (Variables|Default|SetInGameWidget _returnvalue))
  (UserInterface|Viewport|AddtoViewport _output_get 0))

(event EventOnCollected
  (params (Score :type Integer))
  ;[1 1 1] pickup collect default
  (CallFunction|AddCurrentScore Score))

(fn ConstructionScript)

(fn GetCurrentScore
  (return (Variables|Default|GetCurrentScore)))

(fn SetCurrentScore
  (params (CurrentScore :type Integer))
  (Variables|Default|SetCurrentScore (Math|Integer|Max(Integer) CurrentScore))
  (CallFunction|UpdateScoreonScreen))

(fn AddCurrentScore
  (params (ScoreToAdd :type Integer))
  (CallFunction|SetCurrentScore (+ (Math|Integer|Max(Integer) ScoreToAdd) (CallFunction|GetCurrentScore))))

(fn SetDefaultMazeTemplate
  (params (NewMazeTemplate :type S%20Maze%20Structure))
  (Variables|Default|SetDefaultMazeTemplate NewMazeTemplate))

(fn GetDefaultMazeTemplate
  (return (Variables|Default|GetDefaultMazeTemplate)))

(fn GetCurrentPlayerController
  (return (Variables|Default|GetPlayerControllerRef)))

(fn GetinGameWidget
  (return (Variables|Default|GetInGameWidget)))

(fn DisplayAnimatedTextonScreen
  (params (Entries :type Array%20of%20S%20Animated%20Text%20Entry%20Structures))
  (bind _totalpredictedtime (Default|DisplayAnimatedText (CallFunction|GetinGameWidget) Entries))
  (return _totalpredictedtime))

(fn UpdateScoreonScreen
  (Default|UpdateScore (CallFunction|GetinGameWidget) (Variables|Default|GetCurrentScore)))