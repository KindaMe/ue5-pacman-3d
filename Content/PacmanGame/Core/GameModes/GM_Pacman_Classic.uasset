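; Classic Pac-Man game mode: runs map selection, levels, scoring and the end-of-game leaderboard.
; Levels cycle Pre, In and Post states, possessing pawns for play and adjusting ghost speed by level.
; Mazes rotate across four spawn points derived from nav mesh bounds; the camera blends over before the old maze is destroyed.
; Timers drive Scatter/Chase, pausing for Frightened, while maze delegates feed score, doubling ghost bonuses and win/loss.
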(event Custom|FrightenedTimerEnd
  ;[0.5606 0.5103 1] handling maze delegates
  ;;[1 1 1] pickups
  (CallFunction|SetGhostModes (Variables|Default|GetCurrentGhostMode))
  (CallFunction|ResumeModeLoopTimer)
  (Class|AudioManagerSubsystem|PlayPowerUpEndSound (Subsystems|GetAudioManagerSubsystem)))

(event Custom|PossessPawns
  ;[1 1 1] possess unpossess pawns
  (Class|GameModeBasePacman|PossessPacman (Class|Maze|GetPacman (Variables|Default|GetMazeRef)))
  (Class|GameModeBasePacman|PossessGhosts (Class|Maze|GetGhosts (Variables|Default|GetMazeRef))))

(event Custom|SpawnPlaceholderMazeAndSetViewTarget
  ;[1 0 0] placeholder to smooth out camera transition while loading first maze
  (bind _returnvalue (Game|SpawnActorfromClass "/Game/PacmanGame/Maze/BP_Maze_Game.BP_Maze_Game_C" (Math|Transform|MakeTransform (Utilities|Array|Get(acopy) (Variables|Default|GetMazeSpawnPoints) (Math|Integer|%(Integer) (- (Variables|Default|GetCurrentLevel) 1) (Utilities|Array|Length (Variables|Default|GetMazeSpawnPoints)))) "0, 0, 0" "1.000000,1.000000,1.000000") "AlwaysSpawn" "MultiplyWithRoot" 0 (Class|GameModeBasePacman|GetMazeTemplate) 0))
  (bind _output_get (Variables|Default|SetMazeRef _returnvalue))
  (Rendering|SetActorHiddenInGame _output_get true)
  (Game|Player|SetViewTargetwithBlend (Class|GameModeBasePacman|GetCurrentPlayerController) _output_get 0.0 "VTBlend_Linear" 0.0 false))

(event Custom|StopModeLoopTimer
  (bind _switchmodetimerhandle (Variables|Default|GetSwitchModeTimerHandle))
  ;[1 1 1] game states
  ;;[1 1 1] mode loop timer
  (if (Utilities|Time|IsValidTimerHandle _switchmodetimerhandle)
    (Utilities|Time|ClearandInvalidateTimerbyHandle _switchmodetimerhandle)))

(event Custom|PauseModeLoopTimer
  (bind _switchmodetimerhandle (Variables|Default|GetSwitchModeTimerHandle))
  ;[1 1 1] game states
  ;;[1 1 1] mode loop timer
  (if (Utilities|Time|IsValidTimerHandle _switchmodetimerhandle)
    (Utilities|Time|PauseTimerbyHandle _switchmodetimerhandle)))

(event Custom|ResumeModeLoopTimer
  (bind _switchmodetimerhandle (Variables|Default|GetSwitchModeTimerHandle))
  ;[1 1 1] game states
  ;;[1 1 1] mode loop timer
  (if (Utilities|Time|IsValidTimerHandle _switchmodetimerhandle)
    (Utilities|Time|UnpauseTimerbyHandle _switchmodetimerhandle)))

(event Custom|OnAnyPickupCollected_Event
  (params (Pickup :type Pickup%20Object%20Reference) (Score :type Integer) (PickupsLeft :type Integer))
  ;[0.5606 0.5103 1] handling maze delegates
  ;;[1 1 1] pickups
  (Class|GameModeBasePacman|IncreaseCurrentScore Score)
  (if (== 0 PickupsLeft)
    (Class|GameModeBasePacman|PostGame true)))

(event Custom|OnPacmanIsDead_Event
  (params (Pacman :type My%20Pawn%20Pacman%20Object%20Reference) (bIsDead :type Boolean))
  ;[0.5606 0.5103 1] handling maze delegates
  ;;[1 1 1] pawns
  (if bIsDead
    (Class|GameModeBasePacman|PostGame false)))

(event Custom|OnGhostIsDead_Event
  (params (Ghost :type My%20Pawn%20Ghost%20Object%20Reference) (bIsDead :type Boolean))
  (bind _deadghosts (Variables|Default|GetDeadGhosts))
  ;[0.5606 0.5103 1] handling maze delegates
  ;;[1 1 1] pawns
  (if bIsDead
    (Utilities|Array|AddUnique _deadghosts Ghost)
    (Class|GameModeBasePacman|IncreaseCurrentScore (* (Variables|Default|GetGhostsEatenOnSingleFrightenMultiplier) (Variables|Default|GetDefaultPointsForEatingGhost)))
    (Variables|Default|SetGhostsEatenOnSingleFrightenMultiplier (* (Variables|Default|GetGhostsEatenOnSingleFrightenMultiplier) 2))
    (else
      (Utilities|Array|RemoveItem _deadghosts Ghost))))

(event Custom|DisplayLeaderboard
  (bind _outplayercontroller (Class|GameModeBasePacman|GetCurrentPlayerController))
  ;[1 1 1] leaderboard
  (bind (_boutistopscore _outmazetoupdate _outcheckedscore _outleaderboardplace) (Class|GameInstancePacman|CheckScoreAgainstLeaderboard (Variables|Default|GetGameInstance) (Class|GameModeBasePacman|GetMazeTemplate) (Class|GameModeBasePacman|GetCurrentScore)))
  (if _boutistopscore
    (bind _returnvalue (UserInterface|CreateWidget "/Game/PacmanGame/UI/PostGame/WBP_HighScore.WBP_HighScore_C"))
    (EventDispatchers|AssignOnNameEntered _returnvalue (delegate Custom|OnNameEntered_Event))
    (UserInterface|Viewport|AddtoViewport _returnvalue 0)
    (else
      (bind _returnvalue_2 (UserInterface|CreateWidget "/Game/PacmanGame/UI/PostGame/WBP_Leaderboard.WBP_Leaderboard_C" 0 false 0 (Utilities|Struct|BreakMazeData (Class|GameModeBasePacman|GetMazeTemplate))))
      (UserInterface|Viewport|AddtoViewport _returnvalue_2 0)))
  (Input|SetInputModeGameandUI _outplayercontroller 0 "DoNotLock" false true)
  (Variables|/Script/Engine.PlayerController|SetbShowMouseCursor _outplayercontroller true))

(event Custom|OnNameEntered_Event
  (params (Name :type Text))
  ;[1 1 1] leaderboard
  (bind (_outupdatedmaze _outplaceindex) (Class|GameInstancePacman|AddScoretoLeaderboard (Variables|Default|GetGameInstance) (stale Custom|DisplayLeaderboard _outmazetoupdate) (Utilities|Struct|MakeLeaderboardEntryData (Utilities|String|ToString(Text) Name) (stale Custom|DisplayLeaderboard _outcheckedscore)) (stale Custom|DisplayLeaderboard _outleaderboardplace)))
  (bind _returnvalue (UserInterface|CreateWidget "/Game/PacmanGame/UI/PostGame/WBP_Leaderboard.WBP_Leaderboard_C" 0 true _outplaceindex (Utilities|Struct|BreakMazeData _outupdatedmaze)))
  (UserInterface|Viewport|AddtoViewport _returnvalue 0))

(event Custom|OnMapSelectedFromList_Event
  (params (Maze :type Maze%20Data%20Structure))
  (bind _outplayercontroller (Class|GameModeBasePacman|GetCurrentPlayerController))
  (bind _outnavmeshboundsvolume (Class|GameModeBasePacman|GetNavMeshBoundsVolume))
  ;[1 1 1] begin play
  (Class|GameModeBasePacman|SetMazeTemplate Maze)
  (Widget|SetVisibility (Variables|Default|GetMazeListWidgetRef) "Hidden")
  (Input|SetInputModeGameOnly _outplayercontroller true)
  (Variables|/Script/Engine.PlayerController|SetbShowMouseCursor _outplayercontroller false)
  (Utilities|IsValid _outnavmeshboundsvolume
    (:Is%20Valid
      (bind _generatedpoints (CallFunction|SplitNavMeshBoundsInto4MazeSpawnPoints _outnavmeshboundsvolume))
      (Variables|Default|SetMazeSpawnPoints _generatedpoints)
      (CallFunction|SpawnPlaceholderMazeandSetViewTarget)
      (Class|GameModeBasePacman|InitGame))
    (:Is%20Not%20Valid
      (Development|PrintString "no nav mesh in level"))))

(event Custom|StopFrightenedTimer
  (bind _frightenedtimerhandle (Variables|Default|GetFrightenedTimerHandle))
  ;[0.5606 0.5103 1] handling maze delegates
  ;;[1 1 1] pickups
  (if (Utilities|Time|IsValidTimerHandle _frightenedtimerhandle)
    (Utilities|Time|ClearandInvalidateTimerbyHandle _frightenedtimerhandle)))

(event Custom|SpawnMaze
  ;[1 1 1] init maze
  (Utilities|IsValid (Variables|Default|GetMazeRef)
    (:Is%20Valid
      (Variables|Default|SetOldMazeRef (Variables|Default|GetMazeRef)))
    (:Is%20Not%20Valid
      _))
  (bind _returnvalue (Game|SpawnActorfromClass "/Game/PacmanGame/Maze/BP_Maze_Game.BP_Maze_Game_C" (Math|Transform|MakeTransform (Utilities|Array|Get(acopy) (Variables|Default|GetMazeSpawnPoints) (Math|Integer|%(Integer) (Variables|Default|GetCurrentLevel) (Utilities|Array|Length (Variables|Default|GetMazeSpawnPoints)))) "0, 0, 0" "1.000000,1.000000,1.000000") "AlwaysSpawn" "MultiplyWithRoot" 0 (Class|GameModeBasePacman|GetMazeTemplate) 0))
  (EventDispatchers|AssignOnAnyPickupCollected _returnvalue (EventDispatchers|CreateEvent :!event Custom|OnAnyPickupCollected_Event))
  (EventDispatchers|AssignOnPacmanIsDead _returnvalue (EventDispatchers|CreateEvent :!event Custom|OnPacmanIsDead_Event))
  (EventDispatchers|AssignOnGhostIsDead _returnvalue (EventDispatchers|CreateEvent :!event Custom|OnGhostIsDead_Event))
  (bind _output_get (Variables|Default|SetMazeRef _returnvalue))
  (Game|Player|SetViewTargetwithBlend (Class|GameModeBasePacman|GetCurrentPlayerController) _output_get (Variables|Default|GetCameraBlend%20Time) "VTBlend_Linear" 0.0 false)
  (Utilities|Time|SetTimerbyEvent (delegate Custom|FinishSpawnMaze) (Variables|Default|GetCameraBlend%20Time)))

(event Custom|InitGhostsBasedOnLevel
  ;[1 1 1] init ghosts
  (for _array_element (Class|Maze|GetGhosts (Variables|Default|GetMazeRef))
    (Class|MyPawn|SetSpeedMultiplier _array_element (+ (/ (- (Variables|Default|GetCurrentLevel) 1) 10) 1.0))))

(event Custom|SetGhostModes
  (params (NewMode :type EGhostMode%20Enum :default "Scatter"))
  ;[1 1 1] set ghost modes
  (for _array_element (Class|Maze|GetGhosts (Variables|Default|GetMazeRef))
    (if (not (Utilities|Array|ContainsItem (Variables|Default|GetDeadGhosts) _array_element))
      (bind _asbp_pawn_ghost (Utilities|Casting|CastToBP_Pawn_Ghost _array_element))
      (Default|ChangeMode _asbp_pawn_ghost NewMode)))
  (switch Utilities|FlowControl|Switch|SwitchonEGhostMode NewMode
    (:Scatter
      (Class|InGameWidget|DisplayAnimatedText (Class|GameModeBasePacman|GetinGameWidget) (Utilities|Array|MakeArray (Utilities|Struct|MakeAnimatedTextEntry "CALM" 0.0 0.5 "(R=1.000000,G=1.000000,B=1.000000,A=1.000000)") (Utilities|Struct|MakeAnimatedTextEntry "DOWN" 0.25 0.75 "(R=0.000000,G=1.000000,B=0.000000,A=1.000000)")) false))
    (:Chase
      (Class|InGameWidget|DisplayAnimatedText (Class|GameModeBasePacman|GetinGameWidget) (Utilities|Array|MakeArray (Utilities|Struct|MakeAnimatedTextEntry "RUN" 0.0 0.75 "(R=1.000000,G=0.000000,B=0.000000,A=1.000000)")) false))
    (:Frightened
      (Class|InGameWidget|DisplayAnimatedText (Class|GameModeBasePacman|GetinGameWidget) (Utilities|Array|MakeArray (Utilities|Struct|MakeAnimatedTextEntry "MAKE" 0.0 0.5 "(R=1.000000,G=1.000000,B=1.000000,A=1.000000)") (Utilities|Struct|MakeAnimatedTextEntry "THEM" 0.25 0.5 "(R=1.000000,G=1.000000,B=1.000000,A=1.000000)") (Utilities|Struct|MakeAnimatedTextEntry "PAY" 0.5 0.75 "(R=1.000000,G=0.000000,B=0.000000,A=1.000000)")) false))))

(event Custom|StartModeLoopTimer
  ;[1 1 1] game states
  ;;[1 1 1] mode loop timer
  (CallFunction|TimerSwitchtoScatterMode))

(event Custom|FinishSpawnMaze
  (bind _oldmazeref (Variables|Default|GetOldMazeRef))
  ;[1 1 1] init maze
  (Utilities|IsValid _oldmazeref
    (:Is%20Valid
      (Actor|DestroyActor _oldmazeref))
    (:Is%20Not%20Valid
      _))
  (CallFunction|InitGhostsBasedonLevel)
  (Class|GameModeBasePacman|PreGame))

(event Custom|UnPossessPawns
  ;[1 1 1] possess unpossess pawns
  (Class|GameModeBasePacman|UnPossessPacman (Class|Maze|GetPacman (Variables|Default|GetMazeRef)))
  (Class|GameModeBasePacman|UnPossessGhosts (Class|Maze|GetGhosts (Variables|Default|GetMazeRef))))

(event EventBeginPlay
  (bind _outplayercontroller (Class|GameModeBasePacman|GetCurrentPlayerController))
  ;[1 1 1] begin play
  (|CallParentFunction)
  (bind _asbp_game_instance (Utilities|Casting|CastToBP_GameInstance (Game|GetGameInstance)))
  (bind _output_get (Variables|Default|SetGameInstance _asbp_game_instance))
  (bind _returnvalue (UserInterface|CreateWidget "/Game/PacmanGame/UI/PreGame/WBP_MazeList.WBP_MazeList_C" 0 (Variables|/Script/Pacman3D.GameInstancePacman|GetMazes _output_get)))
  (bind _output_get_2 (Variables|Default|SetMazeListWidgetRef _returnvalue))
  (EventDispatchers|AssignOnMapSelectedfromList _output_get_2 (delegate Custom|OnMapSelectedFromList_Event))
  (UserInterface|Viewport|AddtoViewport _output_get_2 0)
  (Input|SetInputModeUIOnly _outplayercontroller 0 "DoNotLock" true)
  (Variables|/Script/Engine.PlayerController|SetbShowMouseCursor _outplayercontroller true))

(event EventPostGame
  (params (bIsWin :type Boolean))
  (bind _currentlevel (Variables|Default|GetCurrentLevel))
  (bind _returnvalue (Utilities|Text|ToText(Integer) _currentlevel))
  ;[1 1 1] game states
  (CallFunction|StopModeLoopTimer)
  (CallFunction|StopFrightenedTimer)
  (CallFunction|UnPossessPawns)
  (if bIsWin
    (bind _outtotalpredictedtime (Class|InGameWidget|DisplayAnimatedText (Class|GameModeBasePacman|GetinGameWidget) (Utilities|Array|MakeArray (Utilities|Struct|MakeAnimatedTextEntry "LEVEL" 0.0 1.0 "(R=1.000000,G=1.000000,B=1.000000,A=1.000000)") (Utilities|Struct|MakeAnimatedTextEntry _returnvalue 0.5 1.0 "(R=1.000000,G=1.000000,B=1.000000,A=1.000000)") (Utilities|Struct|MakeAnimatedTextEntry "COMPLETE" 1.25 1.5 "(R=0.000000,G=1.000000,B=0.000000,A=1.000000)")) true))
    (CallFunction|IncrementLevel)
    (Utilities|Time|SetTimerbyEvent (EventDispatchers|CreateEvent :!event InitGame) (+ _outtotalpredictedtime 1.0))
    (else
      (bind _outtotalpredictedtime_2 (Class|InGameWidget|DisplayAnimatedText (Class|GameModeBasePacman|GetinGameWidget) (Utilities|Array|MakeArray (Utilities|Struct|MakeAnimatedTextEntry "LEVEL" 0.0 1.0 "(R=1.000000,G=1.000000,B=1.000000,A=1.000000)") (Utilities|Struct|MakeAnimatedTextEntry _returnvalue 0.5 1.0 "(R=1.000000,G=1.000000,B=1.000000,A=1.000000)") (Utilities|Struct|MakeAnimatedTextEntry "FAIL" 1.25 1.5 "(R=1.000000,G=0.000000,B=0.000000,A=1.000000)")) true))
      (Utilities|FlowControl|Delay _outtotalpredictedtime_2)
      (bind _outtotalpredictedtime_3 (Class|InGameWidget|DisplayAnimatedText (Class|GameModeBasePacman|GetinGameWidget) (Utilities|Array|MakeArray (Utilities|Struct|MakeAnimatedTextEntry "FINAL" 0.5 1.0 "(R=1.000000,G=1.000000,B=1.000000,A=1.000000)") (Utilities|Struct|MakeAnimatedTextEntry "SCORE" 1.0 1.0 "(R=1.000000,G=1.000000,B=1.000000,A=1.000000)") (Utilities|Struct|MakeAnimatedTextEntry (Utilities|Text|ToText(Integer) (Class|GameModeBasePacman|GetCurrentScore)) 2.0 2.0 "(R=0.000000,G=1.000000,B=0.005000,A=1.000000)")) true))
      (Utilities|FlowControl|Delay _outtotalpredictedtime_3)
      (CallFunction|DisplayLeaderboard))))

(event EventInitGame
  ;[1 1 1] game states
  (CallFunction|SpawnMaze))

(event EventPreGame
  ;[1 1 1] game states
  (bind _outtotalpredictedtime (Class|InGameWidget|DisplayAnimatedText (Class|GameModeBasePacman|GetinGameWidget) (Utilities|Array|MakeArray (Utilities|Struct|MakeAnimatedTextEntry "LEVEL" 1.0 1.0 "(R=1.000000,G=1.000000,B=1.000000,A=1.000000)") (Utilities|Struct|MakeAnimatedTextEntry (Utilities|Text|ToText(Integer) (Variables|Default|GetCurrentLevel)) 1.5 1.0 "(R=1.000000,G=1.000000,B=1.000000,A=1.000000)") (Utilities|Struct|MakeAnimatedTextEntry "START" 2.75 1.0 "(R=0.000000,G=1.000000,B=0.000000,A=1.000000)")) true))
  (Utilities|FlowControl|Delay _outtotalpredictedtime)
  (Class|GameModeBasePacman|InGame))

(event EventInGame
  ;[1 1 1] game states
  (CallFunction|PossessPawns)
  (CallFunction|StartModeLoopTimer))

(event EventFrightenGhosts
  ;[0.5606 0.5103 1] handling maze delegates
  ;;[1 1 1] pickups
  (Class|AudioManagerSubsystem|PlayPowerUpStartSound (Subsystems|GetAudioManagerSubsystem))
  (CallFunction|PauseModeLoopTimer)
  (Variables|Default|SetGhostsEatenOnSingleFrightenMultiplier 1)
  (CallFunction|SetGhostModes "Frightened")
  (bind _returnvalue (Utilities|Time|SetTimerbyEvent (delegate Custom|FrightenedTimerEnd) (Variables|Default|GetDefaultFrightenTime)))
  (Variables|Default|SetFrightenedTimerHandle _returnvalue))

(fn ConstructionScript)

(fn TimerSwitchtoScatterMode
  (bind _output_get (Variables|Default|SetCurrentGhostMode "Scatter"))
  (CallFunction|SetGhostModes _output_get)
  (bind _returnvalue (Utilities|Time|SetTimerbyEvent (EventDispatchers|CreateEvent :!event TimerSwitchtoChaseMode) (Variables|Default|GetDefaultScatterTime)))
  (Variables|Default|SetSwitchModeTimerHandle _returnvalue))

(fn TimerSwitchtoChaseMode
  (bind _output_get (Variables|Default|SetCurrentGhostMode "Chase"))
  (CallFunction|SetGhostModes _output_get)
  (bind _returnvalue (Utilities|Time|SetTimerbyEvent (EventDispatchers|CreateEvent :!event TimerSwitchtoScatterMode) (Variables|Default|GetDefaultChaseTime)))
  (Variables|Default|SetSwitchModeTimerHandle _returnvalue))

(fn IncrementLevel
  (Math|Integer|IncrementInt (Variables|Default|GetCurrentLevel)))

(fn SplitNavMeshBoundsInto4MazeSpawnPoints
  (params (NavMeshBoundsVolume :type Nav%20Mesh%20Bounds%20Volume%20Object%20Reference))
  (bind (_origin _boxextent) (Collision|GetActorBounds NavMeshBoundsVolume false false))
  (bind _returnvalue (Math|Float|Min(Float) (.x _boxextent) (.y _boxextent)))
  (bind _returnvalue_2 (* _returnvalue -1.0))
  (Utilities|IsValid NavMeshBoundsVolume
    (:Is%20Valid
      (LocalVariables|SetLargeSquareCenter _origin)
      (return (Utilities|Array|MakeArray (+ (LocalVariables|GetLargeSquareCenter) (Math|Vector|MakeVector 0.0 0.0 0.0)) (+ (LocalVariables|GetLargeSquareCenter) (Math|Vector|MakeVector _returnvalue_2 0.0 0.0)) (+ (LocalVariables|GetLargeSquareCenter) (Math|Vector|MakeVector _returnvalue_2 _returnvalue_2 0.0)) (+ (LocalVariables|GetLargeSquareCenter) (Math|Vector|MakeVector 0.0 _returnvalue_2 0.0)))))))