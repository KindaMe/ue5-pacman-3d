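; Game mode for classic Pacman that runs the match loop from countdown through play to a win or loss.
; On begin play it takes the last maze template from the game instance, spawns the maze actor and makes it the player's view target.
; After a printed countdown, the player possesses Pacman and ghosts get default controllers.
; PostGame unpossesses all pawns, then loads the menu on a win or respawns the maze on a loss.
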(event Custom|PreGame
  (bind _starttimer (Variables|Default|GetStartTimer))
  (Utilities|FlowControl|Delay 1.0 :!label _label)
  (if (== 0 _starttimer)
    (Development|PrintString "GO!" true true "(R=0.000000,G=0.660000,B=1.000000,A=1.000000)" 1.0)
    (CallFunction|InGame)
    (else
      (Development|PrintString (Utilities|String|ToString(Integer) _starttimer) true true "(R=0.000000,G=0.660000,B=1.000000,A=1.000000)" 1.0)
      (Math|Integer|DecrementInt _starttimer
        (:%20%20
          (goto _label))))))

(event Custom|PossessPawns
  (Pawn|Possess (Variables|Default|GetPlayerControllerRef) (Variables|/Game/PacmanGame/Core/Maze/BP_Maze.BP_Maze_C|GetPacmanPawn (Variables|Default|GetMazeRef)))
  (for _array_element (Variables|/Game/PacmanGame/Core/Maze/BP_Maze.BP_Maze_C|GetGhostPawns (Variables|Default|GetMazeRef))
    (Pawn|SpawnDefaultController _array_element)))

(event Custom|InGame
  (CallFunction|PossessPawns))

(event Custom|RestartGame
  (Variables|Default|SetStartTimer (Variables|GameplayDefaults|GetGameStartCountdownTime))
  (CallFunction|SpawnMaze)
  (CallFunction|PreGame))

(event Custom|SpawnMaze
  (Utilities|IsValid (Variables|Default|GetMazeRef)
    (:Is%20Valid
      (Actor|DestroyActor (Variables|Default|GetMazeRef)))
    (:Is%20Not%20Valid
      _))
  (bind _returnvalue (Game|SpawnActorfromClass "/Game/PacmanGame/Maze/BP_Maze_Game.BP_Maze_Game_C" (Math|Transform|MakeTransform "0, 0, 0" "0, 0, 0" "1.000000,1.000000,1.000000") "AlwaysSpawn" "MultiplyWithRoot" 0 (Variables|Default|GetMazeTemplate) 100 0))
  (Variables|Default|SetMazeRef _returnvalue)
  (Game|Player|SetViewTargetwithBlend (Variables|Default|GetPlayerControllerRef) (Variables|Default|GetMazeRef) 0.0 "VTBlend_Linear" 0.0 false))

(event Custom|PostGame
  (params (IsWin? :type Boolean))
  (if IsWin?
    (Development|PrintString "YOU WIN!")
    (else
      (Development|PrintString "YOU LOST!")))
  (CallFunction|UnPossessPawns)
  (Utilities|FlowControl|Delay 3.0)
  (if IsWin?
    (Default|LoadMenuLevel (Variables|Default|GetGameInstanceRef))
    (else
      (CallFunction|RestartGame))))

(event Custom|UnPossessPawns
  (Pawn|UnPossess (Variables|Default|GetPlayerControllerRef))
  (for _array_element (Variables|/Game/PacmanGame/Core/Maze/BP_Maze.BP_Maze_C|GetGhostPawns (Variables|Default|GetMazeRef))
    (Pawn|UnPossess (AI|GetAIController _array_element))))

(event EventBeginPlay
  (bind _asbp_game_instance (Utilities|Casting|CastToBP_GameInstance (Game|GetGameInstance)))
  (Variables|Default|SetGameInstanceRef _asbp_game_instance)
  (Variables|Default|SetMazeTemplate (Utilities|Array|Get(acopy) (Variables|/Game/PacmanGame/Core/BP_GameInstance.BP_GameInstance_C|GetMazes _asbp_game_instance) (Utilities|Array|LastIndex (Variables|/Game/PacmanGame/Core/BP_GameInstance.BP_GameInstance_C|GetMazes _asbp_game_instance))))
  (CallFunction|RestartGame))

(event EventPostLogin
  (params (NewPlayer :type Player%20Controller%20Object%20Reference))
  (Variables|Default|SetPlayerControllerRef NewPlayer))

(fn ConstructionScript)