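; BP_Maze_Editor is an actor Blueprint that generates default maze layout data for the Pacman game.
; Its construction script loops over a Height by Width grid, using IsEdge to add wall cell classes on the border and floor cell classes inside.
; The resulting cell entries, each holding class, row and column, are stored with the dimensions in the Maze struct; no cells are spawned here.
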(event EventBeginPlay
  (|CallParentFunction) ; This node is disabled and will not be called.\nDrag off pins to build functionality.
)

(event Collision|EventActorBeginOverlap
  (params (OtherActor :type Actor%20Object%20Reference))
  (|CallParentFunction OtherActor) ; This node is disabled and will not be called.\nDrag off pins to build functionality.
)

(event EventTick
  (params (DeltaSeconds :type Float%20%28single-precision%29))
  (|CallParentFunction DeltaSeconds) ; This node is disabled and will not be called.\nDrag off pins to build functionality.
)

(fn ConstructionScript
  (bind _width (Variables|Default|GetWidth))
  (bind _height (Variables|Default|GetHeight))
  (bind _returnvalue (- _width 1))
  (bind _returnvalue_2 (- _height 1))
  (for _index (range 0 _returnvalue_2)
    (for _index_2 (range 0 _returnvalue)
      (bind _returnvalue_3 (CallFunction|IsEdge _index_2 _returnvalue _index _returnvalue_2))
      (if _returnvalue_3
        (Utilities|Array|Add (LocalVariables|GetCells) (Utilities|Struct|MakeS_Cell "/Game/PacmanGame/Maze/BP_MazeCell_Wall.BP_MazeCell_Wall_C" _index _index_2))
        (else
          (Utilities|Array|Add (LocalVariables|GetCells) (Utilities|Struct|MakeS_Cell "/Game/PacmanGame/Maze/BP_MazeCell_Floor.BP_MazeCell_Floor_C" _index _index_2))))))
  (Variables|Default|SetMaze (Utilities|Struct|MakeS_Maze "None" (Variables|Default|GetWidth) (Variables|Default|GetHeight) (LocalVariables|GetCells)))
  (|CallParentFunction))

(fn IsEdge
  (params (Width :type Integer) (WidthMax :type Integer) (Height :type Integer) (HeightMax :type Integer))
  (return (or (or (== Width 0) (== Width WidthMax)) (or (== Height 0) (== Height HeightMax)))))