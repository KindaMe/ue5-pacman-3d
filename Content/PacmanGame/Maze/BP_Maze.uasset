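; Pac-Man maze actor that builds the level from a Maze struct of grid cells and their classes.
; The construction script spawns each cell as a child actor component placed and scaled by GridSize, then caches all ghost and Pacman pawns.
; It also centres the spring arm camera and sets its length from the larger maze dimension.
; RefreshMazeTemplate rebuilds the struct from classes the placed child actors report, allowing the layout to be read back.
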(event EventBeginPlay)

(event Collision|EventActorBeginOverlap
  (params (OtherActor :type Actor%20Object%20Reference)))

(event EventTick
  (params (DeltaSeconds :type Float%20%28single-precision%29)))

(fn ConstructionScript
  (bind _gridsize (Variables|Default|GetGridSize))
  (for _array_element (.cells (Variables|Default|GetMaze))
    (bind _returnvalue (AddComponent|AddChildActorComponent false (Math|Transform|MakeTransform (Math|Vector|MakeVector (Math|Conversions|ToFloat(Integer) (* (.gridx _array_element) _gridsize)) (Math|Conversions|ToFloat(Integer) (* (.gridy _array_element) _gridsize)) 0.0) "0, 0, 0" (Math|Conversions|ToVector(Float) (CallFunction|GetGridScaleMultipler)))))
    (ChildActorComponent|SetChildActorClass _returnvalue (.cell _array_element))
    (Utilities|Array|Add (Variables|Default|GetChildActorComponents) (Utilities|Struct|MakeS_ChildActorComponentInfo _returnvalue (.gridx _array_element) (.gridy _array_element))))
  (CallFunction|ResetCameraLocation)
  (CallFunction|FillReferenceArrays))

(fn ResetCameraLocation
  (bind _gridsize (Variables|Default|GetGridSize))
  (bind _maze (Variables|Default|GetMaze))
  (bind _gridsize_2 (Variables|Default|GetGridSize))
  (bind _springarm (Variables|Default|GetSpringArm))
  (bind _returnvalue (/ _gridsize 2))
  (bind _returnvalue_2 (* (.height _maze) _gridsize_2))
  (bind _returnvalue_3 (* (.width _maze) _gridsize_2))
  (Variables|/Script/Engine.SpringArmComponent|SetTargetArmLength _springarm (Math|Conversions|ToFloat(Integer) (Math|Integer|Max(Integer) _returnvalue_3 _returnvalue_2)))
  (Transformation|SetRelativeLocation _springarm (Math|Vector|MakeVector (Math|Conversions|ToFloat(Integer) (- (/ _returnvalue_2 2) _returnvalue)) (Math|Conversions|ToFloat(Integer) (- (/ _returnvalue_3 2) _returnvalue)) 0.0) false false))

(fn RefreshMazeTemplate
  (for _array_element (Variables|Default|GetChildActorComponents)
    (bind _cell (Class|BPICell|GetChildActorClass(Message) (Variables|/Script/Engine.ChildActorComponent|GetChildActor (.component _array_element))))
    (Utilities|Array|Add (LocalVariables|GetCells) (Utilities|Struct|MakeS_Cell _cell (.gridx _array_element) (.gridy _array_element))))
  (bind _output_get (Variables|Default|SetMaze (Utilities|Struct|MakeS_Maze (.Name (Utilities|Struct|BreakS_Maze (Variables|Default|GetMaze))) (.Width (Utilities|Struct|BreakS_Maze (Variables|Default|GetMaze))) (.Height (Utilities|Struct|BreakS_Maze (Variables|Default|GetMaze))) (LocalVariables|GetCells))))
  (return _output_get))

(fn GetGridScaleMultipler
  (return (/ (Variables|Default|GetGridSize) (Variables|Default|GetDefaultGridSize))))

(fn FillReferenceArrays
  (bind _outactors (Actor|GetAllActorsOfClass "/Game/PacmanGame/Characters/Ghosts/Common/BP_Pawn_Ghost.BP_Pawn_Ghost_C"))
  (Variables|Default|SetEnemyPawns _outactors)
  (bind _outactors_2 (Actor|GetAllActorsOfClass "/Game/PacmanGame/Characters/Pacman/BP_Pawn_Pacman.BP_Pawn_Pacman_C"))
  (Variables|Default|SetPlayerPawns _outactors_2))