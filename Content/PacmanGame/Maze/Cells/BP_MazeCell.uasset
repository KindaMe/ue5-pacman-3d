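; BP_MazeCell is a maze cell actor in the Pacman game, built to be spawned through a Child Actor Component.
; It reports its own class and can swap itself for another by setting a new class on its parent component.
; The setter returns whether the class differed, skipping the swap when it matches.
; Event graph and construction script are empty.
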(event EventBeginPlay)

(event Collision|EventActorBeginOverlap
  (params (OtherActor :type Actor%20Object%20Reference)))

(event EventTick
  (params (DeltaSeconds :type Float%20%28single-precision%29)))

(fn ConstructionScript)

(fn GetChildActorClass
  (return (Utilities|GetClass self)))

(fn SetChildActorClass
  (params (Class :type BP%20Maze%20Cell%20Class%20Reference))
  (if (!= Class (Utilities|GetClass self))
    (ChildActorComponent|SetChildActorClass (Class|Actor|GetParentComponent) Class)
    (return true)
    (else
      (return false))))